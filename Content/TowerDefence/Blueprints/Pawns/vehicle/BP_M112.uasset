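; BP_M112 is a vehicle pawn for the tower defence game with a player-aimed turret and gun.
; On BeginPlay it creates the BP_UserInterface widget for the first player controller and adds it to the viewport.
; LookUp and Turn axis input accumulate into gun elevation and turret rotation, clamped to fixed angle limits.
; Custom events store both angles, and nothing in these graphs applies them to the mesh.
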(event `Elevation`
  (params (GunElevation :type "Float (double-precision)"))
  (set `self.GunElevation` GunElevation))

(event `self.ReceiveBeginPlay`
  (bind _returnvalue (`|CreateWidget` "/Game/TowerDefence/Interface/BP_UserInterface.BP_UserInterface_C" (`GameplayStatics.GetPlayerController` 0)))
  (`UserWidget.AddToViewport` _returnvalue 0))

(event `SetTurretRotation`
  (params (TurretRotation :type "Float (double-precision)"))
  (set `self.TurretRotation` TurretRotation))

(event `InputAxis|LookUp`
  (params (AxisValue :type "Float (single-precision)"))
  (if (!= AxisValue 0.0)
    (`self.Elevation` (`KismetMathLibrary.FClamp` (+ (`self.GunElevation`) AxisValue) -20.0 50.0))))

(event `InputAxis|Turn`
  (params (AxisValue :type "Float (single-precision)"))
  (if (!= AxisValue 0.0)
    (`self.SetTurretRotation` (`KismetMathLibrary.FClamp` (+ AxisValue (`self.TurretRotation`)) -70.0 70.0))))

(fn `UserConstructionScript`)